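; BP_Stand is a puzzle target in a VR game that advances the room once all cubes sit on it.
; CheckCubes, which nothing here calls, tests every BP_Cube's location against X and Y ranges offset from the stand's origin; the Y upper bound derives from the stand's Z.
; If all pass, it spawns a BP_Button at a fixed location and increments the VRPawn's Room counter.
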(event EventBeginPlay)

(event Collision|EventActorBeginOverlap
  (params (OtherActor :type Actor%20Object%20Reference)))

(event EventTick
  (params (DeltaSeconds :type Float%20%28single-precision%29)))

(fn ConstructionScript)

(fn CheckCubes
  (bind _returnvalue (Transformation|GetActorLocation))
  (Variables|Default|SetAllCubesIn true)
  (bind _outactors (Actor|GetAllActorsOfClass "/Game/GameContent/Blueprints/BP_Cube.BP_Cube_C"))
  (for _array_element _outactors
    (if (Math|Float|InRange(Float) (.x (Transformation|GetActorLocation _array_element)) (.x _returnvalue) (+ (.x _returnvalue) 3e+01))
      (if (not (Math|Float|InRange(Float) (.y (Transformation|GetActorLocation _array_element)) (.y _returnvalue) (+ (.z _returnvalue) 35.0)))
        (Variables|Default|SetAllCubesIn false))
      (else
        (Variables|Default|SetAllCubesIn false))))
  (if (Variables|Default|GetAllCubesIn)
    (Game|SpawnActorfromClass "/Game/GameContent/Blueprints/BP_Button.BP_Button_C" (Math|Transform|MakeTransform "500.000000,50.000000,120.000000" "0, 0, 0" "1.000000,1.000000,1.000000") "Undefined" "MultiplyWithRoot" 0 0)
    (bind _returnvalue_2 (Actor|GetActorOfClass "/Game/VRTemplate/Blueprints/VRPawn.VRPawn_C"))
    (Variables|/Game/VRTemplate/Blueprints/VRPawn.VRPawn_C|SetRoom _returnvalue_2 (+ (Variables|/Game/VRTemplate/Blueprints/VRPawn.VRPawn_C|GetRoom _returnvalue_2) 1))))